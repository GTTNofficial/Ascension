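; Player controller that creates the HUD widget on begin play and handles the inventory toggle input.
; The Inventory action casts the player to GameplayCharacter and shows or hides its InventoryRef, switching input mode and mouse cursor and setting the character's IsInventoryOpen flag.
; An older WeaponInventoryTemp widget setup remains in the graph but is never run.
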(event `self.ReceiveBeginPlay`
  (`|ExecutionSequence`
    (:`then_0`
      ;[1 1 1] Creazione widget
      (bind _returnvalue (`|CreateWidget` "/Game/Blueprints/Character/HUD.HUD_C"))
      (`/Engine/EditorBlueprintResources/StandardMacros.IsValid` _returnvalue
        (:`Is Valid`
          (`UserWidget.AddToViewport` _returnvalue 0)
          (set `self.HUD` _returnvalue))))))

(event `InputAction|Inventory`
  (params (Key :type "Key Structure" :default "AnyKey"))
  ;[1 1 1] Keybinding inventario
  (:`Pressed`
    (bind _asgameplay_character (cast `/Game/Blueprints/Character/GameplayCharacter` (`GameplayStatics.GetPlayerCharacter` 0)))
    (bind _inventoryref (`/Game/Blueprints/Character/GameplayCharacter.InventoryRef` _asgameplay_character))
    (if (`/Game/Blueprints/Inventory/Blueprints/BP_Inventory.isVisible?` _inventoryref)
      (`/Game/Blueprints/Inventory/Blueprints/BP_Inventory.HideInventory` _inventoryref)
      (`WidgetBlueprintLibrary.SetInputMode_GameOnly` self)
      (set `self.bShowMouseCursor` false)
      (set `/Game/Blueprints/Character/GameplayCharacter.isInventoryOpen?` false _asgameplay_character)
      (else
        (`/Game/Blueprints/Inventory/Blueprints/BP_Inventory.ShowInventory` _inventoryref)
        (`WidgetBlueprintLibrary.SetInputMode_GameAndUIEx` self (`/Game/Blueprints/Inventory/Blueprints/BP_Inventory.MainWidget` _inventoryref) "DoNotLock" false)
        (set `self.bShowMouseCursor` true)
        (set `/Game/Blueprints/Character/GameplayCharacter.isInventoryOpen?` true _asgameplay_character)))))

(fn `UserConstructionScript`)