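; BP_Chest is an interactable inventory chest that highlights on focus through custom depth, clearing it after a one-second delay.
; On BeginPlay, non-authority instances spawn a BP_Storage linked to the first player character and generate its slot widgets.
; Closing hides that storage, but interaction only prints a debug "Hello" on remotes.
; The show-storage logic and an old backup are disconnected.
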(event `BeginFocus`
  (`PrimitiveComponent.SetRenderCustomDepth` (`self.StaticMesh`) true)
  (`KismetSystemLibrary.Delay` 1.0)
  (`self.EndFocus`))

(event `EndFocus`
  (`PrimitiveComponent.SetRenderCustomDepth` (`self.StaticMesh`) false))

(event `OnStorageClosed`
  (bind _storageactor (`self.StorageActor`))
  (`/Engine/EditorBlueprintResources/StandardMacros.IsValid` _storageactor
    (:`Is Valid`
      (`/Game/Blueprints/Inventory/Blueprints/BP_Storage.HideStorage` _storageactor))))

(event `OnInteract`
  (params (Character :type "/Game/Blueprints/Character/GameplayCharacter Object Reference"))
  (`/Engine/EditorBlueprintResources/ActorMacros.Switch Has Authority`
    (:`Remote`
      (`KismetSystemLibrary.PrintString` "Hello"))))

(event `CreateStorage`
  (`/Engine/EditorBlueprintResources/ActorMacros.Switch Has Authority` :!label _label
    (:`Remote`
      (bind _asgameplay_character (cast `/Game/Blueprints/Character/GameplayCharacter` (`GameplayStatics.GetPlayerCharacter` 0)))
      (bind _output_get (set `self.CharacterRef` _asgameplay_character))
      (bind _returnvalue (`|SpawnActorFromClass` "/Game/Blueprints/Inventory/Blueprints/BP_Storage.BP_Storage_C" (`KismetMathLibrary.MakeTransform` (0.0 0.0 0.0)) "AlwaysSpawn" "OverrideRootScale" null (`self.AmountOfSlots`) _output_get (`self.SlotsPerRow`) self))
      (bind _output_get_2 (set `self.StorageActor` _returnvalue))
      (`/Game/Blueprints/Inventory/Widget/StorageWidget.GenerateSlotWidgets` (`/Game/Blueprints/Inventory/Blueprints/BP_Storage.StorageWidget` _output_get_2) _output_get_2))))

(event `self.ReceiveBeginPlay`
  (goto _label))

(fn `UserConstructionScript`)