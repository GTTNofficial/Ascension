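; Base weapon actor that a GameplayCharacter can pick up, carry on its body and drop.
; InteractPickUp registers the weapon in the character's inventory, marks it equipped, calls its own Drop if flagged, then attaches it to a fixed mesh socket per returned slot.
; Drop detaches the weapon and enables physics and collision without changing the inventory.
; Focus events toggle custom depth rendering on the weapon mesh.
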(event `Drop`
  (bind _weaponstaticmesh (`self.WeaponStaticMesh`))
  ;[1 1 1] Droppa l'arma NON modifica l'inventario
  (`self.K2_DetachFromActor` "KeepWorld" "KeepWorld" "KeepWorld") ; Droppa
  (`PrimitiveComponent.SetSimulatePhysics` _weaponstaticmesh true) ; Simula fisica
  (`PrimitiveComponent.SetCollisionEnabled` _weaponstaticmesh "QueryAndPhysics") ; Abilita collisioni
)

(event `AttachWeaponToCharacter`
  (params (Socket :type Name))
  ;[1 1 1] Attach al player
  (bind _asgameplay_character (cast `/Game/Blueprints/Character/GameplayCharacter` (`self.GetOwner`)))
  (bind _mesh (`Character.Mesh` _asgameplay_character))
  (if (`SceneComponent.DoesSocketExist` _mesh Socket)
    (`self.K2_AttachToComponent` _mesh Socket "SnapToTarget" "KeepRelative" "KeepRelative")))

(event `InteractPickUp`
  (params (Owner :type "Character Object Reference"))
  ;[1 1 1] Pickup arma
  (if (not (`self.isEquipped`))
    (bind _asgameplay_character (cast `/Game/Blueprints/Character/GameplayCharacter` Owner))
    (bind (_slot _drop_) (`/Game/Blueprints/Character/GameplayCharacter.AddWeaponToInventory` _asgameplay_character self)) ; Trovo uno slot libero
    (bind _output_get (set `self.Slot` _slot)) ; Setto lo slot dell'arma
    (set `self.isEquipped` true) ; Equip = true, non può essere raccolta
    (if _drop_
      (`self.Drop`))
    (`self.SetOwner` Owner)
    (switch `int` _output_get ; I socket per ora sono statici
      (:`1`
        (`self.AttachWeaponToCharacter` "S_Weapon1"))
      (:`2`
        (`self.AttachWeaponToCharacter` "S_Weapon2"))
      (:`3`
        (`self.AttachWeaponToCharacter` "S_Weapon3") ; Pistola
      ))))

(event `BeginFocus`
  ;[1 1 1] Pickup arma
  (`PrimitiveComponent.SetRenderCustomDepth` (`self.WeaponStaticMesh`) true))

(event `EndFocus`
  ;[1 1 1] Pickup arma
  (`PrimitiveComponent.SetRenderCustomDepth` (`self.WeaponStaticMesh`) false))

(fn `UserConstructionScript`)